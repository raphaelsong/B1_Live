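; Player controller that owns the score HUD and shows the game result screen.
; On begin play it creates the score widget and passes it the clear score from BP_B1GameMode.
; Score and retry-count events update that widget.
; Game over and game clear open a result widget with failure or success, and a clear also spawns a congratulation actor at the player pawn.
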(event `self.ReceiveBeginPlay`
  (`|ExecutionSequence`
    (:`then_0`
      (bind _returnvalue (`|CreateWidget` "/Game/UI/WBP_PlayerScore.WBP_PlayerScore_C" self))
      (bind _output_get (set `self.PlayerScoreWidget` _returnvalue))
      (`UserWidget.AddToViewport` _output_get 0))
    (:`then_1`
      (bind _asbp_b1game_mode (cast `/Game/Blueprints/BP_B1GameMode` (`GameplayStatics.GetGameMode`)))
      (`/Game/UI/WBP_PlayerScore.SetClearScore` (`self.PlayerScoreWidget`) (`B1GameMode.ClearScore` _asbp_b1game_mode)))))

(event `self.K2_OnScoreChanged`
  (params (NewScore :type Integer))
  (`/Game/UI/WBP_PlayerScore.SetScore` (`self.PlayerScoreWidget`) NewScore))

(event `self.K2_GameOver`
  (`self.GameResult` false))

(event `self.K2_GameClear`
  (`|ExecutionSequence`
    (:`then_0`
      (`self.GameResult` true))
    (:`then_1`
      (`|SpawnActorFromClass` "/Game/UI/BP_Congratulation.BP_Congratulation_C" (`self.GetTransform` (`GameplayStatics.GetPlayerPawn` 0)) "Undefined" "MultiplyWithRoot" null null))))

(event `self.K2_GameRetryCount`
  (params (NewRetryCount :type Integer))
  (`/Game/UI/WBP_PlayerScore.SetRetryCount` (`self.PlayerScoreWidget`) NewRetryCount))

(fn `GameResult`
  (params (InSuccess :type Boolean))
  (bind _returnvalue (`|CreateWidget` "/Game/UI/WBP_GameResult.WBP_GameResult_C" self))
  (`UserWidget.AddToViewport` _returnvalue 0)
  (`/Game/UI/WBP_GameResult.SetResult` _returnvalue (`local.InSuccess`)))

(fn `UserConstructionScript`)